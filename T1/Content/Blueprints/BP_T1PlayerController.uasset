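; BP_T1PlayerController is a player controller that lets the player cycle control between the BP_T1Character actors in the level.
; BeginPlay gathers those characters into the T1Characters array.
; Pressing the 1 key calls ChangeCharacter, which unpossesses the current pawn and possesses the character at CharacterIndex if that index is valid.
; The index then increments and wraps by modulo of the array length.
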(event `self.ReceiveBeginPlay`
  (bind _outactors (`GameplayStatics.GetAllActorsOfClass` "/Game/Blueprints/BP_T1Character.BP_T1Character_C"))
  (set `self.T1Characters` _outactors))

(event `Key|One`
  (params (Key :type "Key Structure"))
  (:`Pressed`
    (`self.ChangeCharacter` (`self.CharacterIndex`))
    (bind _result (`/Engine/EditorBlueprintResources/StandardMacros.IncrementInt` (`self.CharacterIndex`))
      (:`  `
        (set `self.CharacterIndex` (mod _result (`KismetArrayLibrary.Array_Length` (`self.T1Characters`))))))))

(fn `ChangeCharacter`
  (params (Index :type Integer))
  (`self.UnPossess`)
  (if (`KismetArrayLibrary.Array_IsValidIndex` (`self.T1Characters`) Index)
    (`self.Possess` (`|GetArrayItem` (`self.T1Characters`) (`local.Index`)))))

(fn `UserConstructionScript`)