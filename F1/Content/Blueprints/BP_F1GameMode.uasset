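; Game mode that provides random spawning of red and blue F1 targets at trigger box locations.
; BeginPlay caches every TriggerBox in the level and starts a looping one-second timer, presumably bound to RandomSpawnTarget.
; RandomSpawnTarget makes a weighted roll that favors blue over the rarer red target, then spawns it at a randomly chosen box's transform.
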(event `self.ReceiveBeginPlay`
  (bind _outactors (`GameplayStatics.GetAllActorsOfClass` "/Script/Engine.TriggerBox"))
  (set `self.TriggerBoxes` _outactors)
  (`KismetSystemLibrary.K2_SetTimerDelegate` (`|CreateDelegate` :!event `RandomSpawnTarget`) 1.0 true))

(fn `RandomSpawnTarget`
  (`|ExecutionSequence`
    (:`then_0`
      (if (<= (`KismetMathLibrary.RandomFloatInRange` 0.0 100.0) 20.0)
        (set `self.SpawnActorClass` "/Game/Blueprints/BP_F1TargetRed.BP_F1TargetRed_C")
        (else
          (set `self.SpawnActorClass` "/Game/Blueprints/BP_F1TargetBlue.BP_F1TargetBlue_C"))))
    (:`then_1`
      (`|SpawnActorFromClass` (`self.SpawnActorClass`) (`self.GetTransform` (`|GetArrayItem` (`self.TriggerBoxes`) (`KismetMathLibrary.RandomIntegerInRange` 0 (- (`KismetArrayLibrary.Array_Length` (`self.TriggerBoxes`)) 1)))) "Undefined" "MultiplyWithRoot" null null))))

(fn `UserConstructionScript`)